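; Post-effect controller that switches the screen look between Default and Chase modes and drains color as stamina runs low.
; CallDefault and CallChase set the mode and toggle blend weights on two post-process settings sources, PEDefault and PEChase.
; Tick updates the active mode, scaling saturation by a squared stamina ratio below half of the maximum fed through SetStamina.
; Chase mode waits a few ticks before applying its gamma tint and desaturation.
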(event EventBeginPlay)

(event Collision|EventActorBeginOverlap
  (params (OtherActor :type Actor%20Object%20Reference)))

(event EventTick
  (params (DeltaSeconds :type Float%20%28single-precision%29))
  (switch Utilities|FlowControl|Switch|SwitchonPOSTEFFECT (Variables|Default|Getposttype)
    (:NewEnumerator0
      (CallFunction|ProcessDefault))
    (:NewEnumerator1
      (CallFunction|ProcessChase))))

(fn ConstructionScript)

(fn AllClear
  (Variables|/Script/Engine.PostProcessComponent|SetBlendWeight (Variables|Default|GetPE_Chase) 0.0)
  (Variables|/Script/Engine.PostProcessComponent|SetBlendWeight (Variables|Default|GetPE_Default) 0.0))

(fn CallChase
  (CallFunction|AllClear)
  (Variables|/Script/Engine.PostProcessComponent|SetBlendWeight (Variables|Default|GetPE_Chase) 1.0)
  (Variables|Default|Setposttype "NewEnumerator1"))

(fn CallDefault
  (CallFunction|AllClear)
  (Variables|/Script/Engine.PostProcessComponent|SetBlendWeight (Variables|Default|GetPE_Default) 1.0)
  (Variables|Default|Setposttype "NewEnumerator0"))

(fn ProcessDefault
  (bind _stamina_now (Variables|Default|GetStamina_now))
  (bind _stamina_max (Variables|Default|GetStamina_MAX))
  (bind _returnvalue (* _stamina_max 0.5))
  (bind _returnvalue_2 (/ _stamina_now _returnvalue))
  (bind _returnvalue_3 (Math|Float|Power _returnvalue_2 2.0))
  (Variables|Default|SetCount_Time_Chase 0)
  (if (< _stamina_now _returnvalue)
    (Utilities|Struct|SetmembersinPostProcessSettings (Variables|/Script/Engine.PostProcessComponent|GetSettings (Variables|Default|GetPE_Default)) (Math|Vector4|MakeVector4 _returnvalue_3 _returnvalue_3 _returnvalue_3 1.0))))

(fn ProcessChase
  (bind _stamina_now (Variables|Default|GetStamina_now))
  (bind _stamina_max (Variables|Default|GetStamina_MAX))
  (bind _pe_chase (Variables|Default|GetPE_Chase))
  (bind _returnvalue (* _stamina_max 0.5))
  (bind _settings (Variables|/Script/Engine.PostProcessComponent|GetSettings _pe_chase))
  (bind _returnvalue_2 (/ _stamina_now _returnvalue))
  (bind _returnvalue_3 (Math|Float|Power _returnvalue_2 2.0))
  (bind _result (Math|Integer|IncrementInt (Variables|Default|GetCount_Time_Chase))
    (:%20%20
      (Variables|Default|SetCount_Time_Chase _result)
      (if (not (< (Variables|Default|GetCount_Time_Chase) 10))
        (Utilities|Struct|SetmembersinPostProcessSettings _settings (Math|Vector4|MakeVector4 0.63 0.6 0.6 0.6))
        (if (< _stamina_now _returnvalue)
          (Utilities|Struct|SetmembersinPostProcessSettings _settings (Math|Vector4|MakeVector4 _returnvalue_3 _returnvalue_3 _returnvalue_3 1.0)))))))

(fn SetStamina
  (params (now :type Float%20%28double-precision%29) (max :type Float%20%28double-precision%29))
  (Variables|Default|SetStamina_now now)
  (Variables|Default|SetStamina_MAX max))