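; BP_KeyDOOR is a door actor that opens once every actor in SwitchTargets has been destroyed.
; BeginPlay binds each target's OnDestroyed to remove it from the list, playing OpenDoorTimeLine when none remain to slide the door with sinusoidal easing.
; A Delay-throttled Tick countdown runs regardless of door state, periodically reversing the timeline to close it.
; ShowItemId and ShowItemName expose item information.
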(event Custom|TryOpenDoor
  (params (DestroyedActor :type Actor%20Object%20Reference))
  (Utilities|Array|RemoveItem (Variables|セットアップ|GetSwitchTargets) DestroyedActor)
  (if (Utilities|Array|IsEmpty (Variables|セットアップ|GetSwitchTargets))
    (CallFunction|OpenDoor)))

(event Custom|OpenDoor
  (Utilities|FlowControl|Sequence
    (:then_0
      (bind _alpha (Timeline|OpenDoorTimeLine Play)
        (:Update
          (Transformation|SetRelativeTransform (Variables|コンポーネント|GetDoor) (Math|Transform|MakeTransform (Math|Vector|MakeVector 0.0 (Math|Interpolation|Ease "SinusoidalInOut" _alpha 0.0 154.0) 0.0) "0.000000,-90.000000,0.000000" "1.300000,1.000000,1.300000") false false))))
    (:then_1
      (Variables|Default|SetIsOpen true))))

(event EventBeginPlay
  (for _array_element (Variables|セットアップ|GetSwitchTargets)
    (Game|BindEventtoOnDestroyed _array_element (delegate Custom|TryOpenDoor))))

(event Collision|EventActorBeginOverlap
  (params (OtherActor :type Actor%20Object%20Reference)))

(event EventTick
  (params (DeltaSeconds :type Float%20%28single-precision%29))
  (Utilities|FlowControl|Delay 1.0)
  (if (== (Variables|Default|GetSeconds) 0)
    (Variables|Default|SetSeconds 3)
    (Variables|Default|SetIsOpen false)
    (bind _alpha (Timeline|OpenDoorTimeLine Reverse)
      (:Update
        (Transformation|SetRelativeTransform (Variables|コンポーネント|GetDoor) (Math|Transform|MakeTransform (Math|Vector|MakeVector 0.0 (Math|Interpolation|Ease "SinusoidalInOut" _alpha 0.0 154.0) 0.0) "0.000000,-90.000000,0.000000" "1.300000,1.000000,1.300000") false false)))
    (else
      (Variables|Default|SetSeconds (- (Variables|Default|GetSeconds) 1)))))

(fn ConstructionScript)

(fn ShowItemId
  (return "None"))

(fn ShowItemName
  (return (Variables|Default|GetItemName)))